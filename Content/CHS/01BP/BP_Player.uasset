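; Player character for a side-scrolling game, moving along world X with Y pinned every tick.
; An air jump launches it forward and up, and its single charge resets while not falling.
; BeginPlay turns the mesh materials into dynamic instances, which the wet state tints blue or resets to white.
; Entering water sets that state and triggers an HP loss event on BP_Instance, while UpdateWet reapplies the current tint.
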(event `self.ReceiveBeginPlay`
  (for (_array_element _array_index) (`MeshComponent.GetMaterials` (`self.Mesh`))
    (bind _returnvalue (`KismetMaterialLibrary.CreateDynamicMaterialInstance` _array_element (`KismetStringLibrary.Conv_StringToName` (`KismetStringLibrary.Conv_IntToString` _array_index))))
    (`KismetSystemLibrary.PrintString` (`KismetStringLibrary.Conv_IntToString` _array_index))
    (`KismetArrayLibrary.Array_Insert` (`self.PlayerMaterials`) _returnvalue _array_index)
    (`PrimitiveComponent.SetMaterial` (`self.Mesh`) _array_index _returnvalue)))

(event `InWaterEvent`
  (set `self.isWet` true)
  (`/Game/CHS/01BP/BP_Instance.Instance_LoseHP_Event` (cast `/Game/CHS/01BP/BP_Instance` (`GameplayStatics.GetGameInstance`) :!pure true))
  (for _array_element (`self.PlayerMaterials`) :!label _label
    (`/Engine/EditorBlueprintResources/StandardMacros.IsValid` _array_element
      (:`Is Valid`
        (`MaterialInstanceDynamic.SetVectorParameterValue` _array_element "ChangeColor" (struct :`R` 0.183775 :`G` 0.225965 :`B` 0.869792 :`A` 1.0))))))

(event `UpdateWet`
  (if (`self.isWet`)
    (goto _label)
    (else
      (for _array_element (`self.PlayerMaterials`) :!label _label_2
        (`/Engine/EditorBlueprintResources/StandardMacros.IsValid` _array_element
          (:`Is Valid`
            (`MaterialInstanceDynamic.SetVectorParameterValue` _array_element "ChangeColor" (struct :`R` 1.0 :`G` 1.0 :`B` 1.0 :`A` 1.0))))))))

(event `OutWaterEvent`
  (set `self.isWet` false)
  (goto _label_2))

(event `InputAxis|우로이동`
  (params (AxisValue :type "Float (single-precision)"))
  (`self.AddMovementInput` (`KismetMathLibrary.MakeVector` (`self.Speed`)) AxisValue))

(event `InputAxis|좌로이동`
  (params (AxisValue :type "Float (single-precision)"))
  (`self.AddMovementInput` (`KismetMathLibrary.MakeVector` (`self.Speed`)) AxisValue))

(event `InputAction|점프`
  (params (Key :type "Key Structure"))
  (bind _returnvalue_x (`KismetMathLibrary.BreakVector` (`SceneComponent.GetForwardVector` (`self.CapsuleComponent`))))
  (:`Pressed`
    (`self.Jump`)
    (if (and (!= (`self.JumpNum`) 0) (`NavMovementComponent.IsFalling` (`self.CharacterMovement`)))
      (`/Engine/EditorBlueprintResources/StandardMacros.DecrementInt` (`self.JumpNum`)
        (:`  `
          (`self.LaunchCharacter` (+ (* (`KismetMathLibrary.Normal` (`KismetMathLibrary.MakeVector` _returnvalue_x)) 300.0) (0.0 0.0 600.0)) true))))))

(event `self.ReceiveTick`
  (params (DeltaSeconds :type "Float (single-precision)"))
  (bind (_returnvalue_x _returnvalue_y _returnvalue_z) (`KismetMathLibrary.BreakVector` (`self.K2_GetActorLocation`)))
  ;[1 1 1] Y위치 고정
  (`self.K2_SetActorLocation` (`KismetMathLibrary.MakeVector` _returnvalue_x 880.0 _returnvalue_z))
  (if (not (`NavMovementComponent.IsFalling` (`self.CharacterMovement`)))
    (set `self.JumpNum` 1)))

(fn `UserConstructionScript`)