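; BP_NPC is an NPC that shows a dialogue widget while the player stands in its Box trigger.
; On overlap with BP_Player, it creates a UMG_DIEDialog in its Widget component and passes it the current TextNum and itself.
; TextNum then increments, so each new entry requests the next text index with no bound check here.
; Leaving the box clears the widget.
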(event `self.Box.OnComponentBeginOverlap`
  (params (OverlappedComponent :type "PrimitiveComponent Object Reference") (OtherActor :type "Actor Object Reference") (OtherComp :type "PrimitiveComponent Object Reference") (OtherBodyIndex :type Integer) (bFromSweep :type Boolean) (SweepResult :type "HitResult Structure (by ref)"))
  (bind _textnum (`self.TextNum`))
  (cast `/Game/CHS/01BP/BP_Player` OtherActor)
  (bind _returnvalue (`|CreateWidget` "/Game/CHS/05UI/UMG_DIEDialog.UMG_DIEDialog_C"))
  (`WidgetComponent.SetWidget` (`self.Widget`) _returnvalue)
  (`/Game/CHS/05UI/UMG_DIEDialog.UpdateText` _returnvalue _textnum self)
  (bind _result (`/Engine/EditorBlueprintResources/StandardMacros.IncrementInt` _textnum)
    (:`  `
      (set `self.TextNum` _result))))

(event `self.Box.OnComponentEndOverlap`
  (params (OverlappedComponent :type "PrimitiveComponent Object Reference") (OtherActor :type "Actor Object Reference") (OtherComp :type "PrimitiveComponent Object Reference") (OtherBodyIndex :type Integer))
  (cast `/Game/CHS/01BP/BP_Player` OtherActor)
  (`WidgetComponent.SetWidget` (`self.Widget`) null))

(fn `UserConstructionScript`)