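; BP_Monster is a simple wandering monster that roams along the X axis around its spawn location.
; A Tick-driven state machine waits in Idle, picks a random X offset from the start, then walks there at a fixed per-frame step while smoothly turning toward it.
; The Die state, which nothing in this graph sets, destroys the actor after a delay.
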(event `self.ReceiveBeginPlay`
  (set `self.StartLocation` (`self.K2_GetActorLocation`)))

(event `self.ReceiveTick`
  (params (DeltaSeconds :type "Float (single-precision)"))
  (bind _returnvalue (`self.K2_GetActorLocation`))
  (bind _state (`self.State`))
  (bind _targetlocation (`self.TargetLocation`))
  (bind _returnvalue_x (`KismetMathLibrary.BreakVector` (- _targetlocation _returnvalue)))
  (switch `/Game/CHS/01BP/BPE_MonsterState` _state
    (:`NewEnumerator0`
      (`KismetSystemLibrary.Delay` (`self.WaitingTime`))
      (if (not (`|EnumEquality` _state "NewEnumerator2"))
        (set `self.TargetLocation` (+ (`self.StartLocation`) (`KismetMathLibrary.MakeVector` (`KismetMathLibrary.RandomFloatInRange` -200.0 200.0))))
        (set `self.State` "NewEnumerator1")))
    (:`NewEnumerator1`
      (`self.K2_SetActorLocationAndRotation` (+ (`self.K2_GetActorLocation`) (* (`KismetMathLibrary.Normal` (`KismetMathLibrary.MakeVector` _returnvalue_x)) (`self.Speed`))) (`KismetMathLibrary.RLerp` (`self.K2_GetActorRotation`) (`KismetMathLibrary.FindLookAtRotation` _returnvalue _targetlocation) 0.15))
      (if (== (`self.K2_GetActorLocation`) (`self.TargetLocation`) :`ErrorTolerance` (/ (`self.Speed`) 2.0))
        (set `self.State` "NewEnumerator0")))
    (:`NewEnumerator2`
      (`KismetSystemLibrary.Delay` 30.0)
      (`self.K2_DestroyActor`))))

(fn `UserConstructionScript`)