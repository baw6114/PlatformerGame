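; BP_Instance holds the player's coin count and HP, likely as a Game Instance, and broadcasts changes to both.
; Its events add to coins or decrement HP, then fire the matching dispatcher with the new value.
; Losing HP also prints a debug string and fires a game-over dispatcher once HP reaches zero or below.
; A reset event restores coins and HP to their starting values without broadcasting.
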(event `Instance_SetCoin_Event`
  (params (CurCoin :type Integer))
  (bind _output_get (set `self.CurCoin` (+ CurCoin (`self.CurCoin`))))
  (`self.Instance_SetCoin` _output_get))

(event `Instance_LoseHP_Event`
  (bind _curhp (`self.CurHP`))
  (bind _result (`/Engine/EditorBlueprintResources/StandardMacros.DecrementInt` _curhp)
    (:`  `
      (bind _output_get (set `self.CurHP` _result))
      (`self.Instance_LoseHP` _output_get)
      (`KismetSystemLibrary.PrintString` "Lose")
      (if (<= _curhp 0)
        (`self.Instance_GameOver`)))))

(event `ResetVar`
  (set `self.CurCoin` 0)
  (set `self.CurHP` 3))